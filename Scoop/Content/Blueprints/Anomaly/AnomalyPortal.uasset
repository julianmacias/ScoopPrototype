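; AnomalyPortal is a work-in-progress portal actor with an active flag and a Target reference, apparently meant to teleport characters.
; Each Tick tests the Target's position against the portal plane using a dot product and line-plane intersection, detecting front-to-back crossings.
; The crossing result is unused: TeleportActor only saves a ScoopCharacter's velocity and is never called here.
; Render-target and ForceTick functions are empty stubs.
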(event EventBeginPlay)

(event Collision|EventActorBeginOverlap
  (params (OtherActor :type Actor%20Object%20Reference)))

(event EventTick
  (params (DeltaSeconds :type Float%20%28single-precision%29))
  (bind _target (Variables|Default|GetTarget))
  (bind _defaultsceneroot (Variables|Default|GetDefaultSceneRoot))
  (bind _returnvalue (Transformation|GetActorTransform _target))
  (bind _returnvalue_2 (Transformation|GetWorldTransform _defaultsceneroot))
  (bind _returnvalue_3 (Math|Vector|GetForwardVector (.rotation _returnvalue_2)))
  (CallFunction|IsPointinFrontOfPortal (.location _returnvalue) (.location _returnvalue_2) _returnvalue_3)
  (CallFunction|IsPointCrossingPortal (.location _returnvalue) (.location _returnvalue_2) _returnvalue_3))

(fn ConstructionScript)

(fn IsActive
  (return (Variables|Default|Getb_IsActive)))

(fn SetActive
  (params (NewActive :type Boolean))
  (Variables|Default|Setb_IsActive NewActive))

(fn CleanRTT)

(fn SetRTT)

(fn ForceTick)

(fn GetTarget
  (return (Variables|Default|GetTarget)))

(fn SetTarget
  (params (NewTarget :type Actor%20Object%20Reference))
  (Variables|Default|SetTarget NewTarget))

(fn IsPointinFrontOfPortal
  (params (Point :type Vector) (PortalLocation :type Vector) (PortalNormal :type Vector))
  (return (>= (Math|Vector|DotProduct (Math|Vector|Normalize (- Point PortalLocation)) PortalNormal) 0.0)))

(fn IsPointCrossingPortal
  (params (Point :type Vector) (PortalLocation :type Vector) (PortalNormal :type Vector))
  (bind _returnvalue (- Point PortalLocation))
  (bind _returnvalue_2 (Math|Vector|Normalize _returnvalue))
  (bind _returnvalue_3 (Math|Vector|DotProduct _returnvalue_2 PortalNormal))
  (LocalVariables|SetPortalDot _returnvalue_3)
  (LocalVariables|SetIsCrossing false)
  (LocalVariables|SetIsInFront (>= _returnvalue_3 0.0))
  (LocalVariables|SetIsIntersect (.ReturnValue (Class|KismetMathLibrary|LinePlaneIntersectionOriginNormal (Variables|Default|GetLastPosition) Point PortalLocation PortalNormal)))
  (if (Math|Boolean|ANDBoolean (LocalVariables|GetIsIntersect) (not (LocalVariables|GetIsInFront)) (Variables|Default|GetLastInFront))
    (LocalVariables|SetIsCrossing true))
  (Variables|Default|SetLastInFront (LocalVariables|GetIsInFront))
  (Variables|Default|SetLastPosition Point)
  (return (LocalVariables|GetIsCrossing)))

(fn TeleportActor
  (params (ActorToTeleport :type Actor%20Object%20Reference))
  (if (or (== ActorToTeleport 0) (== (Variables|Default|GetTarget) 0))
    (return)
    (else
      (LocalVariables|SetSavedVelocity "0, 0, 0")
      (LocalVariables|SetSC 0)
      (bind _asscoop_character (Utilities|Casting|CastToScoopCharacter ActorToTeleport))
      (bind _output_get (LocalVariables|SetSC _asscoop_character))
      (LocalVariables|SetSavedVelocity (Variables|/Script/Engine.MovementComponent|GetVelocity (Variables|/Script/Engine.Character|GetCharacterMovement _output_get))))))