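; Door actor built from a grid of mesh fragments that animates when the player enters its open trigger.
; The construction script spawns the Width-by-Height grid and records each fragment's original position.
; A timeline scales fragments by index-staggered amounts and lerps them between their grid slots and the upper left or right corner.
; Any overlap with the close trigger reverses the timeline.
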(event OnComponentBeginOverlap(OpenTrigger)
  (params (OverlappedComponent :type Primitive%20Component%20Object%20Reference) (OtherActor :type Actor%20Object%20Reference) (OtherComp :type Primitive%20Component%20Object%20Reference) (OtherBodyIndex :type Integer) (bFromSweep :type Boolean) (SweepResult :type Hit%20Result%20Structure%20%28by%20ref%29))
  (bind _height (Variables|Default|GetHeight))
  (bind _returnvalue (Math|Conversions|ToFloat(Integer) _height))
  (bind _returnvalue_2 (* _returnvalue 5e+01))
  (bind _returnvalue_3 (+ _returnvalue_2 25.0))
  (if (== OtherActor (Game|GetPlayerCharacter 0))
    (bind _scl (Timeline|ScaleTimeline Play)
      (:Update
        (for (_array_element _array_index) (Variables|Default|GetDoor%20Fragments)
          (Transformation|SetWorldScale3D _array_element (* (Variables|Default|GetFragmentScale) (Math|Float|MapRangeClamped _scl 0.01 1.0 (* (* _array_index 0.1) 0.4) 1.0)))
          (if (< (.x (Utilities|Array|Get(acopy) (Variables|Default|GetOriginalLocations) _array_index)) 0.0)
            (Transformation|SetRelativeLocation _array_element (Math|Vector|Lerp(Vector) (Math|Vector|MakeVector -1.5e+02 0.0 _returnvalue_3) (Math|Vector|MakeVector (.x (Utilities|Array|Get(acopy) (Variables|Default|GetOriginalLocations) _array_index)) 0.0 (.z (Utilities|Array|Get(acopy) (Variables|Default|GetOriginalLocations) _array_index))) _scl) false true)
            (else
              (Transformation|SetRelativeLocation _array_element (Math|Vector|Lerp(Vector) (Math|Vector|MakeVector 1.5e+02 0.0 _returnvalue_3) (Math|Vector|MakeVector (.x (Utilities|Array|Get(acopy) (Variables|Default|GetOriginalLocations) _array_index)) 0.0 (.z (Utilities|Array|Get(acopy) (Variables|Default|GetOriginalLocations) _array_index))) _scl) false true))))))))

(event OnComponentBeginOverlap(CloseTrigger)
  (params (OverlappedComponent :type Primitive%20Component%20Object%20Reference) (OtherActor :type Actor%20Object%20Reference) (OtherComp :type Primitive%20Component%20Object%20Reference) (OtherBodyIndex :type Integer) (bFromSweep :type Boolean) (SweepResult :type Hit%20Result%20Structure%20%28by%20ref%29))
  (bind _height (Variables|Default|GetHeight))
  (bind _returnvalue (Math|Conversions|ToFloat(Integer) _height))
  (bind _returnvalue_2 (* _returnvalue 5e+01))
  (bind _returnvalue_3 (+ _returnvalue_2 25.0))
  (bind _scl (Timeline|ScaleTimeline Reverse)
    (:Update
      (for (_array_element _array_index) (Variables|Default|GetDoor%20Fragments)
        (Transformation|SetWorldScale3D _array_element (* (Variables|Default|GetFragmentScale) (Math|Float|MapRangeClamped _scl 0.01 1.0 (* (* _array_index 0.1) 0.4) 1.0)))
        (if (< (.x (Utilities|Array|Get(acopy) (Variables|Default|GetOriginalLocations) _array_index)) 0.0)
          (Transformation|SetRelativeLocation _array_element (Math|Vector|Lerp(Vector) (Math|Vector|MakeVector -1.5e+02 0.0 _returnvalue_3) (Math|Vector|MakeVector (.x (Utilities|Array|Get(acopy) (Variables|Default|GetOriginalLocations) _array_index)) 0.0 (.z (Utilities|Array|Get(acopy) (Variables|Default|GetOriginalLocations) _array_index))) _scl) false true)
          (else
            (Transformation|SetRelativeLocation _array_element (Math|Vector|Lerp(Vector) (Math|Vector|MakeVector 1.5e+02 0.0 _returnvalue_3) (Math|Vector|MakeVector (.x (Utilities|Array|Get(acopy) (Variables|Default|GetOriginalLocations) _array_index)) 0.0 (.z (Utilities|Array|Get(acopy) (Variables|Default|GetOriginalLocations) _array_index))) _scl) false true)))))))

(event EventBeginPlay)

(fn ConstructionScript
  (bind _width (Variables|Default|GetWidth))
  (for _index (range 0 (Variables|Default|GetHeight))
    (for _index_2 (range 0 _width)
      (bind _returnvalue (AddComponent|AddStaticMeshComponent false (Math|Transform|MakeTransform (Math|Vector|MakeVector (- (* (Math|Conversions|ToFloat(Integer) _index_2) 5e+01) (* (* _width 0.5) 5e+01)) 0.0 (+ (* (Math|Conversions|ToFloat(Integer) _index) 5e+01) 25.0)) "0, 0, 0" (Variables|Default|GetFragmentScale))))
      (Utilities|Array|Add (Variables|Default|GetDoor%20Fragments) _returnvalue)
      (Utilities|Array|Add (Variables|Default|GetOriginalLocations) (Math|Vector|MakeVector (- (* (Math|Conversions|ToFloat(Integer) _index_2) 5e+01) (* (* _width 0.5) 5e+01)) 0.0 (+ (* (Math|Conversions|ToFloat(Integer) _index) 5e+01) 25.0))))))