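; BP_PortalActivator is a trigger volume that switches a set of portals on only while the player's character is inside it.
; On BeginPlay it deactivates every portal in its PortalsToActivate array.
; Overlap begin and end events on the Activator component, filtered by a cast to PortalCharacter, call SetActive on each listed portal to enable or disable it.
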(event OnComponentBeginOverlap(Activator)
  (params (OverlappedComponent :type Primitive%20Component%20Object%20Reference) (OtherActor :type Actor%20Object%20Reference) (OtherComp :type Primitive%20Component%20Object%20Reference) (OtherBodyIndex :type Integer) (bFromSweep :type Boolean) (SweepResult :type Hit%20Result%20Structure%20%28by%20ref%29))
  ;[0.1952 1 0] Activate/Deactivate when the character is within the Portal Activator
  (Utilities|Casting|CastToPortalCharacter OtherActor)
  (for _array_element (Variables|Portals|GetPortalsToActivate)
    (Class|Portal|SetActive _array_element true)))

(event OnComponentEndOverlap(Activator)
  (params (OverlappedComponent :type Primitive%20Component%20Object%20Reference) (OtherActor :type Actor%20Object%20Reference) (OtherComp :type Primitive%20Component%20Object%20Reference) (OtherBodyIndex :type Integer))
  ;[0.1952 1 0] Activate/Deactivate when the character is within the Portal Activator
  (Utilities|Casting|CastToPortalCharacter OtherActor)
  (for _array_element (Variables|Portals|GetPortalsToActivate)
    (Class|Portal|SetActive _array_element false)))

(event EventBeginPlay
  ;[0.02595 0 1] Deactivate all portals on begin play within this activator.
  (for _array_element (Variables|Portals|GetPortalsToActivate)
    (Class|Portal|SetActive _array_element false)))

(fn ConstructionScript)